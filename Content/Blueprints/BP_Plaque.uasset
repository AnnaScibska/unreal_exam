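; BP_Plaque is a trigger plate actor that tracks an activated state and shows it through the color of its mesh.
; Any overlap starting on its BoxTrigger sets IsActivated and switches the StaticMesh material to Green.
; When an overlap ends, it waits for a Time delay, then clears IsActivated and turns the mesh Red, but only if IsOperating is true.
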(event `self.BoxTrigger.OnComponentBeginOverlap`
  (params (OverlappedComponent :type "PrimitiveComponent Object Reference") (OtherActor :type "Actor Object Reference") (OtherComp :type "PrimitiveComponent Object Reference") (OtherBodyIndex :type Integer) (bFromSweep :type Boolean) (SweepResult :type "HitResult Structure (by ref)"))
  (set `self.isActivated` true)
  (`PrimitiveComponent.SetMaterial` (`self.StaticMesh`) 0 "/Game/Blueprints/green.green"))

(event `self.BoxTrigger.OnComponentEndOverlap`
  (params (OverlappedComponent :type "PrimitiveComponent Object Reference") (OtherActor :type "Actor Object Reference") (OtherComp :type "PrimitiveComponent Object Reference") (OtherBodyIndex :type Integer))
  (`KismetSystemLibrary.Delay` (`self.time`))
  (if (`self.isOperating`)
    (set `self.isActivated` false)
    (`PrimitiveComponent.SetMaterial` (`self.StaticMesh`) 0 "/Game/Blueprints/red.red")))

(fn `UserConstructionScript`)